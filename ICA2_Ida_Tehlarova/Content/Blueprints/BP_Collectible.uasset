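; BP_Collectible is an interactable pickup that gives the player the box and shows a self-talk line when collected.
; Interact spawns WBP_CollectibleUI with its SelfTalkLine text and sets HasBox on BP_FirstPersonCharacter.
; After a 1.5-second delay it removes the widget and destroys itself.
; GetInteractData returns an empty title and description.
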(event `/Game/Blueprints/Interactable/BPI_Interactable.Interact`
  (bind _returnvalue (`|CreateWidget` "/Game/UI/WBP_CollectibleUI.WBP_CollectibleUI_C"))
  (bind _output_get (set `self.CollectWidget` _returnvalue))
  (`UserWidget.AddToViewport` _output_get 0)
  (`/Game/UI/WBP_CollectibleUI.SetSelfTalkText` _output_get (`self.SelfTalkLine`))
  (bind _asbp_first_person_character (cast `/Game/FirstPerson/Blueprints/BP_FirstPersonCharacter` (`GameplayStatics.GetPlayerCharacter` 0)))
  (set `/Game/FirstPerson/Blueprints/BP_FirstPersonCharacter.hasBox` true _asbp_first_person_character)
  (`KismetSystemLibrary.Delay` 1.5)
  (`Widget.RemoveFromParent` (`self.CollectWidget`))
  (`self.K2_DestroyActor`))

(fn `GetInteractData`
  (returns (Title :type String) (Description :type String))
  (return "" ""))

(fn `UserConstructionScript`)