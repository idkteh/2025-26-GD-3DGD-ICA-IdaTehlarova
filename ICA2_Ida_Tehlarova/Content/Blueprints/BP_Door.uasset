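; BP_Door is a puzzle door that rises when three referenced dials all report being correct.
; CheckPuzzle runs on BeginPlay and is exposed as an event; when all three pass, it plays the DoorOpen timeline.
; Each timeline update lerps from the door's current location toward 200 units above it, so the movement compounds rather than ending at a fixed offset.
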(event `self.ReceiveBeginPlay`
  (`self.CheckPuzzle`))

(event `CheckPuzzle`
  (bind _returnvalue (`self.K2_GetActorLocation`))
  (if (and (`/Game/Blueprints/BP_Dial.IsCorrect` (`self.Dial1Ref`)) (`/Game/Blueprints/BP_Dial.IsCorrect` (`self.Dial2Ref`)) (`/Game/Blueprints/BP_Dial.IsCorrect` (`self.Dial3Ref`)))
    (bind (_direction _alpha) (`Timeline|DoorOpen`)
      (:`Update`
        (`self.K2_SetActorLocation` (`KismetMathLibrary.VLerp` _returnvalue (+ _returnvalue (0.0 0.0 200.0)) _alpha))))))

(fn `UserConstructionScript`)