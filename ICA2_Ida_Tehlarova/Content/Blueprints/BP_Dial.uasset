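; BP_Dial is an interactable puzzle dial that cycles through three values and feeds into a referenced door's puzzle check.
; It evaluates whether its value matches the correct one at BeginPlay and after each turn.
; Interact can be gated on the first-person character holding a box; each turn debug-prints the value and calls CheckPuzzle on the door.
; Its interaction prompt data is empty.
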(event `self.ReceiveBeginPlay`
  (set `self.IsCorrect` (== (`self.CurrentValue`) (`self.CorrectValue`))))

(event `/Game/Blueprints/Interactable/BPI_Interactable.Interact`
  (bind _asbp_first_person_character (cast `/Game/FirstPerson/Blueprints/BP_FirstPersonCharacter` (`GameplayStatics.GetPlayerCharacter` 0)))
  (if (or (not (`self.RequiresBox`)) (`/Game/FirstPerson/Blueprints/BP_FirstPersonCharacter.hasBox` _asbp_first_person_character))
    (bind _output_get (set `self.CurrentValue` (+ (`self.CurrentValue`) 1)))
    (if (== _output_get 3)
      (set `self.CurrentValue` 0))
    (set `self.IsCorrect` (== (`self.CurrentValue`) (`self.CorrectValue`)))
    (`KismetSystemLibrary.PrintString` (`KismetStringLibrary.Conv_IntToString` (`self.CurrentValue`)))
    (`/Game/Blueprints/BP_Door.CheckPuzzle` (`self.DoorRef`))))

(fn `GetInteractData`
  (returns (Title :type String) (Description :type String))
  (return "" ""))

(fn `UserConstructionScript`)